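; Drives the AI date in a dialogue game where the player keeps its engagement meter up until a win timer expires.
; A state machine randomly picks filler, funny, nice or sad lines, then opens a timed reaction window when non-filler dialogue finishes.
; Player laugh events and smile amount adjust the constantly draining engagement according to state.
; Tick updates the meter UI and loads the win or game-over level.
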(event Custom|PlayerLaugh
  (Development|PrintString "HA")
  (switch Utilities|FlowControl|Switch|SwitchonDateAIState (Variables|Default|GetState)
    (:NewEnumerator1
      (CallFunction|AddEngagement -2.0 :!label _label))
    (:NewEnumerator4
      (CallFunction|AddEngagement -1e+01 :!label _label_2))
    (:NewEnumerator3
      (goto _label_2))
    (:NewEnumerator5
      (goto _label))
    (:NewEnumerator2
      (CallFunction|AddEngagement 5.0))
    (:NewEnumerator6
      (goto _label))
    (:NewEnumerator7
      (goto _label))))

(event Custom|DialogueFinish
  ;[1 1 1] Register Event for Dialogue Completion
  ;[1 1 1] On Dialogue finish
  (switch Utilities|FlowControl|Switch|SwitchonDateAIState (Variables|Default|GetState)
    (:NewEnumerator1
      (CallFunction|SwitchState "NewEnumerator0"))
    (:NewEnumerator4
      (CallFunction|SwitchState "NewEnumerator3"))
    (:NewEnumerator5
      (CallFunction|SwitchState "NewEnumerator2"))
    (:NewEnumerator6
      (CallFunction|SwitchState "NewEnumerator7"))))

(event Custom|WidgetCreatedEvent
  ;[1 1 1] Register Event for Dialogue Completion
  (EventDispatchers|BindEventtoDialogueFinish (Variables|/Game/Blueprints/Dialogue/BP_DialogueEvent.BP_DialogueEvent_C|GetDialogueWidgetObj (Variables|Default|GetBP_DialogueEvent)) (delegate Custom|DialogueFinish)))

(event EventBeginPlay
  (EventDispatchers|BindEventtoLaugh (Variables|Default|GetPlayer) (delegate Custom|PlayerLaugh))
  (CallFunction|SwitchState "NewEnumerator0")
  (Variables|Default|SetEngagement (Variables|Default|GetMaxEngagement))
  ;[1 1 1] Make UI
  (bind _returnvalue (UserInterface|CreateWidget "/Game/Blueprints/UI/WB_GameplayUI.WB_GameplayUI_C"))
  (UserInterface|Viewport|AddtoViewport _returnvalue 0)
  (Variables|Default|SetGameplayUI _returnvalue)
  ;[1 1 1] Register Event for Dialogue Completion
  (EventDispatchers|BindEventtoWidgetCreatedEvent (Variables|Default|GetBP_DialogueEvent) (delegate Custom|WidgetCreatedEvent)))

(event EventTick
  (params (DeltaSeconds :type Float%20%28single-precision%29))
  ;[1 1 1] Update UI
  (bind _engagementperentage (CallFunction|GetEngagementPercentage))
  (Default|UpdateEngagementMeter (Variables|Default|GetGameplayUI) _engagementperentage)
  ;[1 1 1] Decrease Engagement
  (CallFunction|AddEngagement (* (* DeltaSeconds (Variables|Default|GetEngagementLossRate)) -1.0))
  ;[1 1 1] Timer
  (Variables|Default|SetCurrentTime (+ (Variables|Default|GetCurrentTime) DeltaSeconds))
  (if (>= (Variables|Default|GetCurrentTime) (Variables|Default|GetTimeToWin))
    ;;[1 1 1] Game Win
    (Game|OpenLevel(byObjectReference) "/Game/Levels/GameWinScreen.GameWinScreen")
    (else
      ;[1 1 1] Check if Game Over
      (if (<= (Variables|Default|GetEngagement) 0.0)
        ;[1 1 1] Game End
        (Game|OpenLevel(byObjectReference) "/Game/Levels/GameOverScreen.GameOverScreen")
        (else
          ;[1 1 1] State Update
          (switch Utilities|FlowControl|Switch|SwitchonDateAIState (Variables|Default|GetState)
            (:NewEnumerator3
              ;[1 1 1] Expecting Frown
              (CallFunction|AddEngagement (* (* -1.0 DeltaSeconds) (Variables|/Game/Blueprints/Player/BP_Bernie.BP_Bernie_C|GetLips%20Val (Variables|Default|GetPlayer)))))
            (:NewEnumerator5
              ;[1 1 1] Talking Funny
              (CallFunction|AddEngagement (* (* 0.2 DeltaSeconds) (Variables|/Game/Blueprints/Player/BP_Bernie.BP_Bernie_C|GetLips%20Val (Variables|Default|GetPlayer)))))
            (:NewEnumerator6
              ;[1 1 1] Expecting Smile
              (CallFunction|AddEngagement (* (* 0.5 DeltaSeconds) (Variables|/Game/Blueprints/Player/BP_Bernie.BP_Bernie_C|GetLips%20Val (Variables|Default|GetPlayer)))))
            (:NewEnumerator7
              ;[1 1 1] Expecting Smile
              (CallFunction|AddEngagement (* (* 1.0 DeltaSeconds) (Variables|/Game/Blueprints/Player/BP_Bernie.BP_Bernie_C|GetLips%20Val (Variables|Default|GetPlayer)))))))))))

(fn ConstructionScript)

(fn GetEngagementPercentage
  (return (/ (Variables|Default|GetEngagement) (Variables|Default|GetMaxEngagement))))

(fn AddEngagement
  (params (Engagement :type Float%20%28double-precision%29))
  (Variables|Default|SetEngagement (Math|Float|Max(Float) (Math|Float|Min(Float) (+ Engagement (Variables|Default|GetEngagement)) (Variables|Default|GetMaxEngagement)) 0.0)))

(fn StartTalkTimer
  (bind _returnvalue (Math|Random|RandomFloatinRange 1.0 4.0))
  (switch int (Math|Random|RandomInteger 4)
    (:0
      (Utilities|Time|SetTimerbyFunctionName 0 "TalkFiller" _returnvalue))
    (:1
      (Utilities|Time|SetTimerbyFunctionName 0 "TalkFunny" _returnvalue))
    (:2
      (Utilities|Time|SetTimerbyFunctionName 0 "TalkSmiley" _returnvalue))
    (:3
      (Utilities|Time|SetTimerbyFunctionName 0 "TalkSad" _returnvalue))))

(fn SwitchState
  (params (NewParam :type DateAIState%20Enum :default "NewEnumerator0"))
  (bind _output_get (Variables|Default|SetState NewParam))
  (switch Utilities|FlowControl|Switch|SwitchonDateAIState _output_get
    (:NewEnumerator0
      (CallFunction|StartTalkTimer))
    (:NewEnumerator3
      (Utilities|Time|SetTimerbyFunctionName 0 "SwitchStateNeutral" (Variables|Default|GetReactionWindow) :!label _label))
    (:NewEnumerator2
      (goto _label))
    (:NewEnumerator7
      (goto _label))))

(fn Talk
  (params (Message :type Dialogue%20Lines%20Structure))
  (bind _stringlines (LocalVariables|GetStringLines))
  (for _array_element (Utilities|Struct|BreakDialogueLines Message)
    (Utilities|Array|Add _stringlines (Utilities|String|ToString(Text) _array_element)))
  (Default|Talk (Variables|Default|GetBP_DialogueEvent) _stringlines))

(fn GetRandomText
  (params (Array :type Array%20of%20Texts))
  (return (Utilities|Array|Get(acopy) Array (Math|Random|RandomInteger (Utilities|Array|Length Array)))))

(fn GetRandomDialogueStruct
  (params (Array :type Array%20of%20Dialogue%20Lines%20Structures))
  (return (Utilities|Array|Get(acopy) Array (Math|Random|RandomInteger (Utilities|Array|Length Array)))))

(fn TalkFiller
  (Variables|Default|SetState "NewEnumerator1")
  (bind _out (CallFunction|GetRandomDialogueStruct (Variables|Default|GetDialogueFiller)))
  (CallFunction|Talk _out))

(fn TalkFunny
  (Variables|Default|SetState "NewEnumerator5")
  (bind _out (CallFunction|GetRandomDialogueStruct (Variables|Default|GetDialogueFunny)))
  (CallFunction|Talk _out))

(fn TalkSad
  (Variables|Default|SetState "NewEnumerator4")
  (bind _out (CallFunction|GetRandomDialogueStruct (Variables|Default|GetDialogueSad)))
  (CallFunction|Talk _out))

(fn TalkSmiley
  (Variables|Default|SetState "NewEnumerator6")
  (bind _out (CallFunction|GetRandomDialogueStruct (Variables|Default|GetDialogueSmiley)))
  (CallFunction|Talk _out))

(fn SwitchStateNeutral
  (CallFunction|SwitchState "NewEnumerator0"))