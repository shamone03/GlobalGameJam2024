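; Player Blueprint for Bernie that turns Lips, Lungs and Throat controls in WB_PlayerUI into body sounds.
; BeginPlay creates the widget, binds its change, click and release events, and adds paused audio components; Tick copies the widget's values.
; Holding Lips plays the stretch sound and release pauses it, while Throat changes during a hold restart the laugh.
; Lungs handlers are empty stubs, leaving inhale and exhale sounds unplayed.
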(event Custom|Handle%20Lips%20Clicked
  (bind _stretch1 (Variables|Default|Getstretch1))
  ;[1 1 1] Lips
  (Class|AudioComponent|SetPaused _stretch1 false)
  (if (not (Audio|Components|Audio|IsPlaying _stretch1))
    (Audio|Components|Audio|Play _stretch1 0.0)))

(event Custom|HandleLipsReleased
  ;[1 1 1] Lips
  (Class|AudioComponent|SetPaused (Variables|Default|Getstretch1) true))

(event Custom|HandleLips
  (params (val :type Float%20%28double-precision%29))
  ;[1 1 1] Lips
)

(event Custom|HandleLungs
  (params (val :type Float%20%28double-precision%29))
  ;[1 1 1] Lungs
)

(event Custom|HandleThroat
  (params (val :type Float%20%28double-precision%29))
  ;[1 1 1] Throat
  (if (Variables|Default|GetisLaughing)
    (Audio|Components|Audio|Play (Variables|Default|Getlaugh1) 0.0)))

(event Custom|HandleThroatClicked
  ;[1 1 1] Throat
  (Variables|Default|SetisLaughing true))

(event Custom|HandleThroatReleased
  ;[1 1 1] Throat
  (Variables|Default|SetisLaughing false))

(event Custom|HandleLungsClicked
  ;[1 1 1] Lungs
)

(event Custom|HandleLungsReleased
  ;[1 1 1] Lungs
)

(event EventBeginPlay
  (bind _returnvalue (Class|InputDeviceLibrary|GetPlayerControllerfromInputDevice))
  (bind _returnvalue_2 (UserInterface|CreateWidget "/Game/Blueprints/Player/WB_PlayerUI.WB_PlayerUI_C" _returnvalue))
  (bind _output_get (Variables|Default|SetplayerUI _returnvalue_2))
  (UserInterface|Viewport|AddtoViewport _output_get 0)
  (EventDispatchers|BindEventtoHandleLipsChanged _output_get (delegate Custom|HandleLips))
  (EventDispatchers|BindEventtoHandleLungsChanged _output_get (delegate Custom|HandleLungs))
  (EventDispatchers|BindEventtoHandleThroatChanged _output_get (delegate Custom|HandleThroat))
  (EventDispatchers|BindEventtoLipsClicked _output_get (delegate Custom|Handle%20Lips%20Clicked))
  (EventDispatchers|BindEventtoLipsReleased _output_get (delegate Custom|HandleLipsReleased))
  (EventDispatchers|BindEventtoLungsClicked _output_get (delegate Custom|HandleLungsClicked))
  (EventDispatchers|BindEventtoLungsReleased _output_get (delegate Custom|HandleLungsReleased))
  (EventDispatchers|BindEventtoThroatClicked _output_get (delegate Custom|HandleThroatClicked))
  (EventDispatchers|BindEventtoThroatReleased _output_get (delegate Custom|HandleThroatReleased))
  ;[1 1 1] Comment
  (bind _returnvalue_3 (AddComponent|AddAudioComponent false))
  (bind _output_get_2 (Variables|Default|Setstretch1 _returnvalue_3))
  (bind _returnvalue_4 (AddComponent|AddAudioComponent false))
  (bind _output_get_3 (Variables|Default|Setlaugh1 _returnvalue_4))
  (bind _returnvalue_5 (AddComponent|AddAudioComponent false))
  (bind _output_get_4 (Variables|Default|Setexhale1 _returnvalue_5))
  (bind _returnvalue_6 (AddComponent|AddAudioComponent false))
  (bind _output_get_5 (Variables|Default|Setinhale1 _returnvalue_6))
  (Class|AudioComponent|SetPaused _output_get_2 true)
  (Class|AudioComponent|SetPaused _output_get_3 true)
  (Class|AudioComponent|SetPaused _output_get_4 true)
  (Class|AudioComponent|SetPaused _output_get_5 true))

(event Collision|EventActorBeginOverlap
  (params (OtherActor :type Actor%20Object%20Reference)))

(event EventTick
  (params (DeltaSeconds :type Float%20%28single-precision%29))
  (bind _playerui (Variables|Default|GetplayerUI))
  (Variables|Default|SetLips%20Val (Variables|/Game/Blueprints/Player/WB_PlayerUI.WB_PlayerUI_C|GetlipsVal _playerui))
  (Variables|Default|SetLungs%20Val (Variables|/Game/Blueprints/Player/WB_PlayerUI.WB_PlayerUI_C|GetlungsVal _playerui))
  (Variables|Default|SetThroat%20Val (Variables|/Game/Blueprints/Player/WB_PlayerUI.WB_PlayerUI_C|GetthroatVal _playerui)))

(fn ConstructionScript)